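; BP_CommonCharacter is a character Blueprint assembled from separate Body, Head and Hair components.
; On BeginPlay it attaches Head and Hair to the Body's "j_kao_wj" socket, keeping world transforms, then plays animation 8_2 once on the Body.
; An unconnected chain would copy left knee and arm socket locations into ABP_Character_Common's IK variables, but it never runs.
; Tick and the construction script are empty.
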(event `self.ReceiveBeginPlay`
  (bind _body (`self.Body`))
  (`SceneComponent.K2_AttachToComponent` (`self.Head`) _body "j_kao_wj" "KeepWorld" "KeepWorld" "KeepWorld" true)
  (`SceneComponent.K2_AttachToComponent` (`self.Hair`) _body "j_kao_wj" "KeepWorld" "KeepWorld" "KeepWorld" true)
  (`SkeletalMeshComponent.PlayAnimation` _body "/Game/8_2.8_2" false))

(event `self.ReceiveTick`
  (params (DeltaSeconds :type "Float (single-precision)")))

(fn `UserConstructionScript`)